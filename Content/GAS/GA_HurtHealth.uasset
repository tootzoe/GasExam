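; GA_HurtHealth is a gameplay ability that applies GE_Damage to a pawn just in front of its avatar.
; On activation it commits, then runs a short forward sphere trace for Pawn objects, ignoring the avatar.
; The hit actor becomes target data for the effect without a hit check, then the ability ends.
; A failed commit cancels the ability.
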(event Ability|EventActivateAbility
  (bind _returnvalue (Ability|GetAvatarActorfromActorInfo))
  (bind _returnvalue_2 (Transformation|GetActorLocation _returnvalue))
  (bind _returnvalue_3 (Ability|CommitAbility))
  (if _returnvalue_3
    (bind _outhit (Collision|SphereTraceForObjects _returnvalue_2 (+ _returnvalue_2 (* (Transformation|GetActorForwardVector _returnvalue) 1e+02)) 0.0 (Utilities|Array|MakeArray "ObjectTypeQuery3") false (Utilities|Array|MakeArray _returnvalue) "None"))
    (GameplayEffects|ApplyGameplayEffectToTarget (Ability|TargetData|AbilityTargetDatafromActor (.hitactor _outhit)) "/Game/GAS/GE_Damage.GE_Damage_C" 1 1)
    (Ability|EndAbility)
    (else
      (Ability|CancelAbility))))

(event Ability|EventOnEndAbility
  (params (bWasCancelled :type Boolean)))