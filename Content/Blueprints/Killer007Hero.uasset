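; Killer007Hero is a playable hero pawn that moves and triggers a health-hurting ability through the Gameplay Ability System.
; BeginPlay adds the Enhanced Input mapping and grants GA_HurtHealth, which IA_Hit activates by its stored handle.
; IA_Move drives movement along the actor's forward and right vectors.
; UpdHealthLabel writes a health value to a TextRender, which is hidden when player controller 0 possesses the hero.
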(event Input|EnhancedActionEvents|EnhancedInputActionIA_Hit
  (params (ActionValue :type Boolean) (ElapsedSeconds :type Float%20%28double-precision%29) (TriggeredSeconds :type Float%20%28double-precision%29) (InputAction :type Input%20Action%20Object%20Reference :default "/Game/Input/IA_Hit.IA_Hit"))
  (Class|AbilitySystemComponent|TryActivateAbility (Variables|Default|GetAbilitySysCompt) (stale EventBeginPlay _returnvalue) true))

(event Input|EnhancedActionEvents|EnhancedInputActionIA_Move
  (params (ActionValue :type Vector%202D%20Structure) (ElapsedSeconds :type Float%20%28double-precision%29) (TriggeredSeconds :type Float%20%28double-precision%29) (InputAction :type Input%20Action%20Object%20Reference :default "/Game/Input/IA_Move.IA_Move"))
  (:Triggered
    (Pawn|Input|AddMovementInput (+ (* (Transformation|GetActorForwardVector) (.x ActionValue)) (* (Transformation|GetActorRightVector) (.y ActionValue))) 1.0 false)))

(event EventBeginPlay
  (Input|AddMappingContext (PlayerController|LocalPlayerSubsystems|GetEnhancedInputLocalPlayerSubsystem (Game|GetPlayerController 0)) "/Game/Input/IMC_Main.IMC_Main" 0 "(bIgnoreAllPressedKeysUntilRelease=True,bForceImmediately=False,bNotifyUserSettings=False)")
  (bind _returnvalue (GameplayAbilities|GiveAbility (Variables|Default|GetAbilitySysCompt) "/Game/GAS/GA_HurtHealth.GA_HurtHealth_C" 0 -1)))

(event Collision|EventActorBeginOverlap
  (params (OtherActor :type Actor%20Object%20Reference)))

(event EventTick
  (params (DeltaSeconds :type Float%20%28single-precision%29)))

(event EventUpdHealthLabel
  (params (Val :type Float%20%28single-precision%29))
  (Rendering|Components|TextRender|SetText (Variables|Default|GetTextRender) (Utilities|Text|ToText(Float) Val "HalfToEven")))

(event EventPossessed
  (params (NewController :type Controller%20Object%20Reference))
  (if (== (Game|GetPlayerController 0) NewController)
    (Rendering|SetVisibility (Variables|Default|GetTextRender) false false)))

(fn ConstructionScript)